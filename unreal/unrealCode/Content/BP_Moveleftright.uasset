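; BP_Moveleftright is an actor that slides its StaticMesh2 component back and forth along its relative X axis.
; Each Tick steps LocationR by a fixed unit and reverses the direction boolean at symmetric limits either side of zero.
; The step ignores delta time, so speed depends on frame rate.
; A Timeline-driven move along Y remains in the graph but never runs.
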(event `self.ReceiveBeginPlay`)

(event `self.ReceiveTick`
  (params (DeltaSeconds :type "Float (single-precision)"))
  (if (`self.오른쪽방향진행`)
    (bind _output_get (set `self.LocationR` (+ (`self.LocationR`) 1.0)))
    (`SceneComponent.K2_SetRelativeLocation` (`self.StaticMesh2`) (`KismetMathLibrary.MakeVector` _output_get) false false)
    (if (>= (`self.LocationR`) 200.0)
      (set `self.오른쪽방향진행` false))
    (else
      (bind _output_get_2 (set `self.LocationR` (+ (`self.LocationR`) -1.0)))
      (`SceneComponent.K2_SetRelativeLocation` (`self.StaticMesh2`) (`KismetMathLibrary.MakeVector` _output_get_2) false false)
      (if (<= (`self.LocationR`) -200.0)
        (set `self.오른쪽방향진행` true)))))

(fn `UserConstructionScript`)