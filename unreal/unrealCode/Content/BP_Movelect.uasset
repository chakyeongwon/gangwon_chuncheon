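; BP_Movelect is an actor that moves a static mesh component continuously around a square path in its local XZ plane.
; Each Tick, a switch on the MoveType enum steps the X or Z offset by a fixed amount, independent of delta time, and sets the mesh's relative location.
; Reaching a square edge advances the state through Right, Up, Left and Down; leftover timeline and boolean-based movement nodes are unconnected.
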(event `self.ReceiveBeginPlay`)

(event `self.ReceiveTick`
  (params (DeltaSeconds :type "Float (single-precision)"))
  (bind _locationrl (`self.LocationRL`))
  (bind _locationrl_2 (`self.LocationRL`))
  (bind _locationud (`self.LocationUD`))
  (bind _locationud_2 (`self.LocationUD`))
  (switch `/Game/EN_MoveType` (`self.MoveType`)
    (:`NewEnumerator0`
      (bind _output_get (set `self.LocationRL` (+ (`self.LocationRL`) 1.0)))
      (`SceneComponent.K2_SetRelativeLocation` (`self.StaticMesh2`) (`KismetMathLibrary.MakeVector` _output_get 0.0 _locationud_2) false false)
      (if (>= _locationrl 200.0)
        (set `self.MoveType` "NewEnumerator1")))
    (:`NewEnumerator1`
      (bind _output_get_2 (set `self.LocationUD` (+ (`self.LocationUD`) 1.0)))
      (`SceneComponent.K2_SetRelativeLocation` (`self.StaticMesh2`) (`KismetMathLibrary.MakeVector` _locationrl 0.0 _output_get_2) false false)
      (if (>= _locationud 200.0)
        (set `self.MoveType` "NewEnumerator2")))
    (:`NewEnumerator2`
      (bind _output_get_3 (set `self.LocationRL` (+ (`self.LocationRL`) -1.0)))
      (`SceneComponent.K2_SetRelativeLocation` (`self.StaticMesh2`) (`KismetMathLibrary.MakeVector` _output_get_3 0.0 _locationud) false false)
      (if (<= _locationrl_2 0.0)
        (set `self.MoveType` "NewEnumerator3")))
    (:`NewEnumerator3`
      (bind _output_get_4 (set `self.LocationUD` (+ (`self.LocationUD`) -1.0)))
      (`SceneComponent.K2_SetRelativeLocation` (`self.StaticMesh2`) (`KismetMathLibrary.MakeVector` _locationrl_2 0.0 _output_get_4) false false)
      (if (<= _locationud_2 0.0)
        (set `self.MoveType` "NewEnumerator0")))))

(fn `UserConstructionScript`)